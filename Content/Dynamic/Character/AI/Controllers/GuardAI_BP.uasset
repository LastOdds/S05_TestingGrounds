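; AI controller for guards that feeds perceived enemies to their behavior tree.
; On BeginPlay it sets up the GuardBehaviourData blackboard, runs GuardBehavior and caches the blackboard component.
; AI perception updates write any sensed actor without the "Npc" tag to the enemy key.
; A failed sense of such an actor clears that key, without checking whether it is the stored enemy.
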(event `self.ReceiveBeginPlay`
  ;[1 1 1] Run Blackboard
  (bind _blackboardcomponent (`self.UseBlackboard` "/Game/Dynamic/Character/AI/Blackboards/GuardBehaviourData.GuardBehaviourData"))
  (`self.RunBehaviorTree` "/Game/Dynamic/Character/AI/BehaviorTrees/RootBehaviors/GuardBehavior.GuardBehavior")
  (set `self.BlackboardComp` _blackboardcomponent))

(event `self.AIPerception.OnTargetPerceptionUpdated`
  (params (Actor :type "Actor Object Reference") (Stimulus :type "AIStimulus Structure"))
  ;[1 1 1] Get Enemy
  (`self.Update Blackboard Enemy Key` Actor Actor Stimulus))

(fn `Update Blackboard Enemy Key`
  (params (`Actor Faction` :type "Actor Object Reference") (`Actor Value` :type "Object Object Reference") (AIStimulus :type "AIStimulus Structure"))
  (bind _enemykey (`self.EnemyKey`))
  (bind _blackboardcomp (`self.BlackboardComp`))
  (if (`self.ActorHasTag` `Actor Faction` "Npc")
    _
    (elif (`.bSuccessfullySensed` (break `AIStimulus` AIStimulus))
      (`BlackboardComponent.SetValueAsObject` _blackboardcomp _enemykey `Actor Value`)
      (else
        (`BlackboardComponent.ClearValue` _blackboardcomp _enemykey)))))

(fn `UserConstructionScript`)