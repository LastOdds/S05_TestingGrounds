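; Tile02_BP is an infinite-terrain tile with an attach transform for chaining, a lockable barrier and a backstop that is hidden on BeginPlay.
; When the player enters the locking volume, the barrier opens and turns green, then after a short delay the backstop restores its collision and toggles visibility.
; On exit, the barrier locks red, InfiniteTerrainGameMode spawns a random tile, and this tile destroys itself shortly after.
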(event `self.ReceiveBeginPlay`
  (`self.HideBackstop`))

(event `self.LockingVolume_0.OnComponentBeginOverlap`
  (params (OverlappedComponent :type "PrimitiveComponent Object Reference") (OtherActor :type "Actor Object Reference") (OtherComp :type "PrimitiveComponent Object Reference") (OtherBodyIndex :type Integer) (bFromSweep :type Boolean) (SweepResult :type "HitResult Structure (by ref)"))
  (`self.IsPlayerActor` OtherActor)
  (`self.Unlock`)
  (`KismetSystemLibrary.Delay` 0.2)
  (`self.UnhideBackstop`))

(event `self.LockingVolume_0.OnComponentEndOverlap`
  (params (OverlappedComponent :type "PrimitiveComponent Object Reference") (OtherActor :type "Actor Object Reference") (OtherComp :type "PrimitiveComponent Object Reference") (OtherBodyIndex :type Integer))
  (`self.IsPlayerActor` OtherActor)
  (`self.Lock`)
  (bind _asinfinite_terrain_game_mode (cast `/Game/Dynamic/GameModes/InfiniteTerrainGameMode` (`GameplayStatics.GetGameMode`)))
  (`/Game/Dynamic/GameModes/InfiniteTerrainGameMode.SpawnRandomTile` _asinfinite_terrain_game_mode)
  (`KismetSystemLibrary.Delay` 0.2)
  (`self.K2_DestroyActor`))

(fn `GetAttachLocation`
  (returns (`Attach Transform` :type "Transform Structure"))
  (return (`SceneComponent.K2_GetComponentToWorld` (`self.AttachPoint_0`))))

(fn `HideBackstop`
  (`SceneComponent.ToggleVisibility` (`self.Backstop`) false)
  (`PrimitiveComponent.SetCollisionEnabled` (`self.Backstop`) "NoCollision"))

(fn `Lock`
  (bind _barrier_0 (`self.Barrier_0`))
  (`PrimitiveComponent.SetCollisionEnabled` _barrier_0 "QueryAndPhysics")
  (`PrimitiveComponent.SetMaterial` _barrier_0 0 "/Game/Dynamic/Tiles/RedBarrier.RedBarrier"))

(fn `UnhideBackstop`
  (`SceneComponent.ToggleVisibility` (`self.Backstop`) false)
  (`PrimitiveComponent.SetCollisionEnabled` (`self.Backstop`) "QueryAndPhysics"))

(fn `Unlock`
  (bind _barrier_0 (`self.Barrier_0`))
  (`PrimitiveComponent.SetCollisionEnabled` _barrier_0 "NoCollision")
  (`PrimitiveComponent.SetMaterial` _barrier_0 0 "/Game/Dynamic/Tiles/GreenBarrier.GreenBarrier"))

(fn `UserConstructionScript`)