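; Tile03_BP is a terrain tile for an infinite terrain game, exposing an attach point transform.
; Its LockingVolume reacts to the player: entry unlocks the green Barrier and, after a short delay, toggles the initially hidden Backstop's visibility and enables its collision.
; Exit relocks the red Barrier, asks InfiniteTerrainGameMode to spawn a random tile, then destroys this tile after a short delay.
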(event `self.ReceiveBeginPlay`
  (`self.HideBackstop`))

(event `self.LockingVolume.OnComponentBeginOverlap`
  (params (OverlappedComponent :type "PrimitiveComponent Object Reference") (OtherActor :type "Actor Object Reference") (OtherComp :type "PrimitiveComponent Object Reference") (OtherBodyIndex :type Integer) (bFromSweep :type Boolean) (SweepResult :type "HitResult Structure (by ref)"))
  (`self.IsPlayerActor` OtherActor)
  (`self.Unlock`)
  (`KismetSystemLibrary.Delay` 0.2)
  (`self.UnhideBackstop`))

(event `self.LockingVolume.OnComponentEndOverlap`
  (params (OverlappedComponent :type "PrimitiveComponent Object Reference") (OtherActor :type "Actor Object Reference") (OtherComp :type "PrimitiveComponent Object Reference") (OtherBodyIndex :type Integer))
  (`self.IsPlayerActor` OtherActor)
  (`self.Lock`)
  (bind _asinfinite_terrain_game_mode (cast `/Game/Dynamic/GameModes/InfiniteTerrainGameMode` (`GameplayStatics.GetGameMode`)))
  (`/Game/Dynamic/GameModes/InfiniteTerrainGameMode.SpawnRandomTile` _asinfinite_terrain_game_mode)
  (`KismetSystemLibrary.Delay` 0.2)
  (`self.K2_DestroyActor`))

(fn `GetAttachLocation`
  (returns (`Attach Transform` :type "Transform Structure"))
  (return (`SceneComponent.K2_GetComponentToWorld` (`self.AttachPoint`))))

(fn `HideBackstop`
  (`SceneComponent.ToggleVisibility` (`self.Backstop`) false)
  (`PrimitiveComponent.SetCollisionEnabled` (`self.Backstop`) "NoCollision"))

(fn `Lock`
  (bind _barrier (`self.Barrier`))
  (`PrimitiveComponent.SetCollisionEnabled` _barrier "QueryAndPhysics")
  (`PrimitiveComponent.SetMaterial` _barrier 0 "/Game/Dynamic/Tiles/RedBarrier.RedBarrier"))

(fn `UnhideBackstop`
  (`SceneComponent.ToggleVisibility` (`self.Backstop`) false)
  (`PrimitiveComponent.SetCollisionEnabled` (`self.Backstop`) "QueryAndPhysics"))

(fn `Unlock`
  (bind _barrier (`self.Barrier`))
  (`PrimitiveComponent.SetCollisionEnabled` _barrier "NoCollision")
  (`PrimitiveComponent.SetMaterial` _barrier 0 "/Game/Dynamic/Tiles/GreenBarrier.GreenBarrier"))

(fn `UserConstructionScript`)