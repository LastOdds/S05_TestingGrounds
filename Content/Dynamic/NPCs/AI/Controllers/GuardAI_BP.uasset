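; AI controller for guard NPCs that runs a behavior tree and reacts to perceived enemies.
; On begin play it sets up the guard blackboard and starts the guard behavior tree.
; Perception updates store any sensed actor without the "Npc" tag as the blackboard enemy, and clear that key when sensing fails.
; Each tick it sets the controlled TPCharacter's Alert and Shooting flags according to whether a valid focus actor exists.
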(event `self.ReceiveBeginPlay`
  ;[1 1 1] Run Blackboard
  (bind _blackboardcomponent (`self.UseBlackboard` "/Game/Dynamic/NPCs/AI/Blackboards/GuardBehaviourData.GuardBehaviourData"))
  (`self.RunBehaviorTree` "/Game/Dynamic/NPCs/AI/BehaviorTrees/RootBehaviors/GuardBehavior.GuardBehavior")
  (set `self.BlackboardComp` _blackboardcomponent))

(event `self.AIPerception.OnTargetPerceptionUpdated`
  (params (Actor :type "Actor Object Reference") (Stimulus :type "AIStimulus Structure"))
  (bind _enemykey (`self.EnemyKey`))
  (bind _blackboardcomp (`self.BlackboardComp`))
  ;[1 1 1] Get Enemy
  (if (`self.ActorHasTag` Actor "Npc")
    _
    (elif (`.bSuccessfullySensed` (break `AIStimulus` Stimulus))
      (`BlackboardComponent.SetValueAsObject` _blackboardcomp _enemykey Actor)
      (else
        (`BlackboardComponent.ClearValue` _blackboardcomp _enemykey)))))

(event `self.ReceiveTick`
  (params (DeltaSeconds :type "Float (single-precision)"))
  ;[1 1 1] Has Valid Focus
  (bind _astpcharacter (cast `/Game/Dynamic/NPCs/Behavior/TPCharacter` (`self.K2_GetPawn`)))
  (bind _output_get (set `/Game/Dynamic/NPCs/Behavior/TPCharacter.Alert` (`KismetSystemLibrary.IsValid` (`self.GetFocusActor`)) _astpcharacter))
  (set `/Game/Dynamic/NPCs/Behavior/TPCharacter.Shooting` _output_get _astpcharacter))

(fn `UserConstructionScript`)