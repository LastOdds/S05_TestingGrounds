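; NPC AI controller Blueprint that runs the Guard_Patrol behavior tree on the PatrolData blackboard.
; Every tick it writes player pawn 0 into the blackboard's EnemyKey, independent of perception.
; AI Perception updates only print a debug string with the controlled pawn, sense class and perceived actor, without feeding the blackboard.
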(event `self.ReceiveBeginPlay`
  (bind _blackboardcomponent (`self.UseBlackboard` "/Game/Static/NPCs/AI/Blackboards/PatrolData.PatrolData"))
  (`self.RunBehaviorTree` "/Game/Static/NPCs/AI/Behavior_Trees/Guard_Patrol.Guard_Patrol")
  (set `self.BlackboardComp` _blackboardcomponent))

(event `self.ReceiveTick`
  (params (DeltaSeconds :type "Float (single-precision)"))
  (`BlackboardComponent.SetValueAsObject` (`self.BlackboardComp`) (`self.EnemyKey`) (`GameplayStatics.GetPlayerPawn` 0)))

(event `self.AIPerception.OnTargetPerceptionUpdated`
  (params (Actor :type "Actor Object Reference") (Stimulus :type "AIStimulus Structure"))
  (bind _returnvalue (`AIPerceptionSystem.GetSenseClassForStimulus` Stimulus))
  (`KismetSystemLibrary.PrintString` (`KismetStringLibrary.Concat_StrStr` (`KismetSystemLibrary.GetObjectName` (`self.K2_GetPawn`)) " " (`KismetSystemLibrary.GetClassDisplayName` _returnvalue) " " (`KismetSystemLibrary.GetDisplayName` Actor))))

(fn `UserConstructionScript`)